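; PlanetAIController_BP is an AI controller that drives teammate characters following or assisting a leader.
; When the teammate option changes, it runs the BT_Teammate behavior tree and writes the leader to the blackboard.
; It then sets the option key to Follow or Assistance.
; For Assistance, it also stores the team's focus enemy as the blackboard enemy.
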(event `self.OnTeammateOptionChanged`
  (params (TeammateOption :type "ETeammateOption Enum" :default "kFollow") (LeaderCharacterPtr :type "CharacterBase Object Reference"))
  (`self.RunBehaviorTree` "/Game/GamePlay/AI/BT_Teammate.BT_Teammate")
  (`|ExecutionSequence`
    (:`then_0`
      (`BlackboardComponent.SetValueAsObject` (`self.Blackboard`) (`self.LeaderPC`) LeaderCharacterPtr))
    (:`then_1`
      (switch `ETeammateOption` TeammateOption
        (:`kFollow`
          (`BlackboardComponent.SetValueAsEnum` (`self.Blackboard`) (`self.TeammateOption`) (enumliteral `/Game/GamePlay/AI/E_TeammateOption` "NewEnumerator0")))
        (:`kAssistance`
          (`BlackboardComponent.SetValueAsEnum` (`self.Blackboard`) (`self.TeammateOption`) (enumliteral `/Game/GamePlay/AI/E_TeammateOption` "NewEnumerator1"))
          (`BlackboardComponent.SetValueAsObject` (`self.Blackboard`) (`self.EnemyPC`) (`self.GetTeamFocusEnemy`)))))))

(fn `UserConstructionScript`)