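; EquipmentTorch_BP is a torch equipment actor that feeds a gravity direction to its Niagara effect.
; Each tick, if its owner is a GravityCharacter, it sets User.GravityDir on KnifeSystemPtr and draws a debug line from the actor along that direction.
; The direction is a difference of two zero vectors, so no character gravity reaches the effect and the line has zero length.
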(event `self.ReceiveTick`
  (params (DeltaSeconds :type "Float (single-precision)"))
  (bind _returnvalue (- (0.0 0.0 0.0) (0.0 0.0 0.0)))
  (bind _asgravity_character (cast `GravityCharacter` (`self.GetOwner`)))
  (`NiagaraComponent.SetNiagaraVariableVec3` (`self.Knife_SystemPtr`) "User.GravityDir" _returnvalue)
  (`KismetSystemLibrary.DrawDebugLine` (`self.K2_GetActorLocation`) (+ (`self.K2_GetActorLocation`) (* _returnvalue 300)) (struct :`G` 0.973958 :`B` 0.406698 :`A` 1.0) 10.0 10.0))

(fn `UserConstructionScript`)